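; BloqueGanador is the winning block that unlocks and ends the level.
; A looping timer polls the game instance's NumeroBloques.
; When it equals one, the cube switches to the accessible material and four boxes lose collision.
; A ThirdPersonCharacter overlapping Box4 opens the post-level selection widget, switches input to UI only and shows the mouse cursor.
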(event OnComponentBeginOverlap(Box4)
  (params (OverlappedComponent :type Primitive%20Component%20Object%20Reference) (OtherActor :type Actor%20Object%20Reference) (OtherComp :type Primitive%20Component%20Object%20Reference) (OtherBodyIndex :type Integer) (bFromSweep :type Boolean) (SweepResult :type Hit%20Result%20Structure%20%28by%20ref%29))
  (Utilities|Casting|CastToThirdPersonCharacter OtherActor)
  (bind _returnvalue (UserInterface|CreateWidget "/Game/UI/WBP_PostLevelSelection.WBP_PostLevelSelection_C"))
  (UserInterface|Viewport|AddtoViewport _returnvalue 0)
  (Input|SetInputModeUIOnly (Game|GetPlayerController 0) _returnvalue "DoNotLock")
  (Variables|/Script/Engine.PlayerController|SetbShowMouseCursor (Game|GetPlayerController 0) true))

(event Custom|WinCondition
  (bind _asmy_gi (Utilities|Casting|CastToMY_GI (Game|GetGameInstance)))
  (if (== (Variables|/Game/Core/MY_GI.MY_GI_C|GetNumeroBloques _asmy_gi) 1)
    (Rendering|Material|SetMaterial (Variables|Default|GetCube) 0 "/Game/Materials/M_BloqueAccesible.M_BloqueAccesible")
    (Collision|SetCollisionEnabled (Variables|Default|GetBox) "NoCollision")
    (Collision|SetCollisionEnabled (Variables|Default|GetBox1) "NoCollision")
    (Collision|SetCollisionEnabled (Variables|Default|GetBox2) "NoCollision")
    (Collision|SetCollisionEnabled (Variables|Default|GetBox3) "NoCollision")))

(event EventBeginPlay
  (Utilities|Time|SetTimerbyEvent (delegate Custom|WinCondition) 0.1 true))

(fn ConstructionScript)